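; Shotgun variant of a chase-player enemy that fires a three-projectile volley when it attacks.
; The Attack event spawns a BP_EnemyProjectile at each of three FireArrow components, using each arrow's world location and rotation, so the arrow placement defines the shot pattern.
; The construction script only calls the parent, and no chase or attack-trigger logic appears in this Blueprint.
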(event EventAttack
  (bind _firearrow2 (Variables|Default|GetFireArrow2))
  (bind _firearrow1 (Variables|Default|GetFireArrow1))
  (bind _firearrow (Variables|Default|GetFireArrow))
  (Game|SpawnActorfromClass "/Game/StudentWork/Weapons/Projectiles/BP_EnemyProjectile.BP_EnemyProjectile_C" (Math|Transform|MakeTransform (Transformation|GetWorldLocation _firearrow) (Transformation|GetWorldRotation _firearrow) "1.000000,1.000000,1.000000") "Undefined" "MultiplyWithRoot" 0 0)
  (Game|SpawnActorfromClass "/Game/StudentWork/Weapons/Projectiles/BP_EnemyProjectile.BP_EnemyProjectile_C" (Math|Transform|MakeTransform (Transformation|GetWorldLocation _firearrow1) (Transformation|GetWorldRotation _firearrow1) "1.000000,1.000000,1.000000") "Undefined" "MultiplyWithRoot" 0 0)
  (Game|SpawnActorfromClass "/Game/StudentWork/Weapons/Projectiles/BP_EnemyProjectile.BP_EnemyProjectile_C" (Math|Transform|MakeTransform (Transformation|GetWorldLocation _firearrow2) (Transformation|GetWorldRotation _firearrow2) "1.000000,1.000000,1.000000") "Undefined" "MultiplyWithRoot" 0 0))

(fn ConstructionScript
  (|CallParentFunction))