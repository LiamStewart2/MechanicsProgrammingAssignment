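; Enemy Blueprint that chases the player and fires projectiles, supplying Move and Attack events.
; Move sends the enemy toward the Player actor with AI MoveTo whenever that reference is valid.
; Attack spawns a BP_EnemyProjectile at the FireArrow component's world location and rotation.
; Nothing in this graph sets Player or calls either event, and the construction script only runs the parent's.
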(event EventMove
  (bind _player (Variables|Default|GetPlayer))
  (Utilities|IsValid _player
    (:Is%20Valid
      (AI|AIMoveTo self "0, 0, 0" _player 5.0 false))))

(event EventAttack
  (bind _firearrow (Variables|Default|GetFireArrow))
  (Game|SpawnActorfromClass "/Game/StudentWork/Weapons/Projectiles/BP_EnemyProjectile.BP_EnemyProjectile_C" (Math|Transform|MakeTransform (Transformation|GetWorldLocation _firearrow) (Transformation|GetWorldRotation _firearrow) "1.000000,1.000000,1.000000") "Undefined" "MultiplyWithRoot" 0 0))

(fn ConstructionScript
  (|CallParentFunction))