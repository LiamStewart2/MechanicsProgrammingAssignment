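; BP_Barrel_Explosion is an explosive barrel that, on its first damage event, flashes and then explodes.
; The construction script creates a dynamic M_Bomb material, and a timeline drives its FlashLevel parameter.
; When the flash finishes, the barrel damages every actor overlapping its sphere, destroys itself and spawns a Niagara explosion effect at its location.
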(event Game|Damage|EventAnyDamage
  (params (Damage :type Float%20%28single-precision%29) (DamageType :type Damage%20Type%20Object%20Reference) (InstigatedBy :type Controller%20Object%20Reference) (DamageCauser :type Actor%20Object%20Reference))
  (Utilities|FlowControl|DoOnce false
    (:Completed
      (bind _flash (Timeline|Flash PlayFromStart)
        (:Update
          (Rendering|Material|SetScalarParameterValue (Variables|Default|GetFlashMaterial) "FlashLevel" _flash :!class /Script/Engine.MaterialInstanceDynamic))
        (:Finished
          (for _array_element (Collision|GetOverlappingActors (Variables|Default|GetSphere) 0 :!class /Script/Engine.PrimitiveComponent)
            (Game|Damage|ApplyDamage _array_element 5.0 0 0))
          (Actor|DestroyActor)
          (Niagara|SpawnSystematLocation "/Game/StudentWork/ParticleSystems/NS_ExplosionEffect.NS_ExplosionEffect" (Transformation|GetActorLocation)))))))

(fn ConstructionScript
  (bind _returnvalue (Rendering|Material|CreateDynamicMaterialInstance (Variables|Default|GetStaticMesh) 0 "/Game/StudentWork/Materials/M_Bomb.M_Bomb" "None" :!class /Script/Engine.PrimitiveComponent))
  (Variables|Default|SetFlashMaterial _returnvalue))