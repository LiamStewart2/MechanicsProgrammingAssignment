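; BP_Door is an interactable double door that slides open when the player character enters its Box trigger.
; The overlap casts to BP_PlayerCharacter and checks HoldingKey, but both outcomes lead to OpenDoor, so the key does not gate it.
; OpenDoor calls separate right and left events, each using MoveComponentTo to ease its mesh sideways in opposite directions.
; No logic closes the door again.
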(event OnComponentBeginOverlap(Box)
  (params (OverlappedComponent :type Primitive%20Component%20Object%20Reference) (OtherActor :type Actor%20Object%20Reference) (OtherComp :type Primitive%20Component%20Object%20Reference) (OtherBodyIndex :type Integer) (bFromSweep :type Boolean) (SweepResult :type Hit%20Result%20Structure%20%28by%20ref%29))
  (bind _asbp_player_character (Utilities|Casting|CastToBP_PlayerCharacter OtherActor))
  (if (Variables|/Game/Blueprints/BP_PlayerCharacter.BP_PlayerCharacter_C|GetHoldingKey _asbp_player_character)
    _
    (else
      _))
  (CallFunction|OpenDoor))

(event Custom|OpenDoor
  (CallFunction|OpenRightDoor)
  (CallFunction|OpenLeftDoor))

(event Custom|OpenLeftDoor
  (Components|MoveComponentTo (Variables|Default|GetLeftDoorMesh) "-80.000000,0.000000,0.000000" "0, 0, 0" false true 2.0 false))

(event Custom|OpenRightDoor
  (Components|MoveComponentTo (Variables|Default|GetRightDoorMesh) "80.000000,0.000000,0.000000" "0, 0, 0" false true 2.0 false))

(fn ConstructionScript)