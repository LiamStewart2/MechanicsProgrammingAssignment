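; BP_Key is a key pickup that stays hidden until the enemies around it are gone.
; It hides its static mesh on BeginPlay and reveals it when an end overlap on EnemyOverlay leaves no BP_EnemyParent actors inside that volume.
; Once the mesh is visible, a BP_PlayerCharacter overlapping KeyPickup gets HoldingKey set to true and the key destroys itself.
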(event OnComponentBeginOverlap(KeyPickup)
  (params (OverlappedComponent :type Primitive%20Component%20Object%20Reference) (OtherActor :type Actor%20Object%20Reference) (OtherComp :type Primitive%20Component%20Object%20Reference) (OtherBodyIndex :type Integer) (bFromSweep :type Boolean) (SweepResult :type Hit%20Result%20Structure%20%28by%20ref%29))
  ;[1 0.08999 0.3318] Player Pickup
  (if (Rendering|IsVisible (Variables|Default|GetStaticMesh))
    (bind _asbp_player_character (Utilities|Casting|CastToBP_PlayerCharacter OtherActor))
    (Variables|/Game/Blueprints/BP_PlayerCharacter.BP_PlayerCharacter_C|SetHoldingKey _asbp_player_character true)
    (Actor|DestroyActor)))

(event OnComponentEndOverlap(EnemyOverlay)
  (params (OverlappedComponent :type Primitive%20Component%20Object%20Reference) (OtherActor :type Actor%20Object%20Reference) (OtherComp :type Primitive%20Component%20Object%20Reference) (OtherBodyIndex :type Integer))
  ;[0.5521 1 0.1042] Check How many Enemies are overallping
  (if (<= (Utilities|Array|Length (Collision|GetOverlappingActors (Variables|Default|GetEnemyOverlay) "/Game/StudentWork/Enemies/AI/BP_EnemyParent.BP_EnemyParent_C" :!class /Script/Engine.PrimitiveComponent)) 0)
    (CallFunction|RevealKey)))

(event Custom|RevealKey
  ;[1 0 0.72] Make static mesh visible
  (Rendering|SetVisibility (Variables|Default|GetStaticMesh) true false))

(event EventBeginPlay
  ;[0.1588 0.8902 1] Hide Key on begin play
  (Rendering|SetVisibility (Variables|Default|GetStaticMesh) false false))

(fn ConstructionScript)