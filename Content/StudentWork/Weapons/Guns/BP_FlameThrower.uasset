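; Flamethrower weapon for a tank that burns objects in a short range ahead of the tank's direction arrow.
; Started spawns the Niagara flame attached to the arrow once, then reactivates that cached system on later uses; Completed deactivates it.
; While triggered, a multi sphere trace along the arrow's forward vector damages every hit, rate-limited by a short timer-reset cooldown.
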(event Custom|ResetCooldown
  (Variables|Default|Setcooldown false))

(event EventTriggered
  (bind _mytank (Variables|Default|GetMyTank))
  (bind _directionarrow (Variables|/Game/Blueprints/BP_PlayerCharacter.BP_PlayerCharacter_C|GetDirectionArrow _mytank))
  (bind _returnvalue (Transformation|GetWorldTransform _directionarrow))
  (if (not (Variables|Default|Getcooldown))
    (bind _outhits (Collision|MultiSphereTraceForObjects (.location _returnvalue) (+ (.location _returnvalue) (* (Math|Vector|GetForwardVector _directionarrow) 2e+02)) 5e+01 (Variables|Default|GetObject%20Types) false 0 "None"))
    (Variables|Default|Setcooldown true)
    (Utilities|Time|SetTimerbyEvent (delegate Custom|ResetCooldown) 0.2)
    (for _array_element _outhits
      (Game|Damage|ApplyDamage (.HitActor (Collision|BreakHitResult _array_element)) 2.0 0 0))))

(event EventStarted
  (Utilities|IsValid (Variables|Default|GetFlameSystem)
    (:Is%20Valid
      (Components|Activation|Activate (Variables|Default|GetFlameSystem) true))
    (:Is%20Not%20Valid
      (bind _returnvalue (Niagara|SpawnSystemAttached "/Game/StudentWork/ParticleSystems/NS_FlamerThrower.NS_FlamerThrower" (Variables|/Game/Blueprints/BP_PlayerCharacter.BP_PlayerCharacter_C|GetDirectionArrow (Variables|Default|GetMyTank)) "None" "0, 0, 0" "0, 0, 0" "KeepRelativeOffset" false))
      (Variables|Default|SetFlameSystem _returnvalue))))

(event EventCompleted
  (Components|Activation|Deactivate (Variables|Default|GetFlameSystem)))

(fn ConstructionScript
  (|CallParentFunction))