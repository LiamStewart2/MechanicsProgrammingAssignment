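; BP_Minigun is a rapid-fire tank gun in the student-work weapons set.
; When Triggered runs, it spawns a BP_Projectile at the location and rotation of the owning tank's DirectionArrow.
; A Cooldown flag cleared after a very short Delay limits the fire rate, so calls during that window are ignored.
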(event EventTriggered
  (bind _mytank (Variables|Default|GetMyTank))
  (bind _directionarrow (Variables|/Game/Blueprints/BP_PlayerCharacter.BP_PlayerCharacter_C|GetDirectionArrow _mytank))
  (if (not (Variables|Default|Getcooldown))
    (Game|SpawnActorfromClass "/Game/StudentWork/Weapons/Projectiles/BP_Projectile.BP_Projectile_C" (Math|Transform|MakeTransform (Transformation|GetWorldLocation _directionarrow) (Transformation|GetWorldRotation _directionarrow) "1.000000,1.000000,1.000000") "Undefined" "MultiplyWithRoot" 0 0)
    (Variables|Default|Setcooldown true)
    (Utilities|FlowControl|Delay 0.05)
    (Variables|Default|Setcooldown false)))

(fn ConstructionScript
  (|CallParentFunction))